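; Bp_Player2 is a player Blueprint that links the player's points and cards to its on-screen UI.
; Each Tick, while the UI is valid, it pushes the points from PlayerComponent into the UI as text.
; ShowCards and HideCards events forward directly to the matching UI calls.
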(event `self.ReceiveBeginPlay`)

(event `self.ReceiveTick`
  (params (DeltaSeconds :type "Float (single-precision)"))
  (if (`KismetSystemLibrary.IsValid` (`self.UI`))
    (`/Game/Player/Bp_WidgetPlayer2.SetPoints` (`self.UI`) (`KismetTextLibrary.Conv_IntToText` (`PlayerComponent.Points` (`self.PlayerComponent`))))))

(event `self.ShowCards`
  (`/Game/Player/Bp_WidgetPlayer2.ShowCards` (`self.UI`)))

(event `self.HideCards`
  (`/Game/Player/Bp_WidgetPlayer2.HideCards` (`self.UI`)))

(fn `UserConstructionScript`)
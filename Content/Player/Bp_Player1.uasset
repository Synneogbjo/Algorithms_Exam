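; Player 1 Blueprint that links its PlayerComponent to the UI for showing points and cards.
; Two seconds after BeginPlay it registers itself with the UI as Player1Ref, then pushes the component's points to the UI every Tick.
; ShowCards asks PlayerComponent for two card indices matching the saved piece's role and passes them to the UI, while HideCards hides them.
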(event `self.ReceiveBeginPlay`
  (`KismetSystemLibrary.Delay` 2.0)
  (set `/Game/Player/Bp_WidgetPlayer.Player1_ref` self (`self.UI`)))

(event `self.ReceiveTick`
  (params (DeltaSeconds :type "Float (single-precision)"))
  (if (`KismetSystemLibrary.IsValid` (`self.UI`))
    (`/Game/Player/Bp_WidgetPlayer.SetPoints` (`self.UI`) (`KismetTextLibrary.Conv_IntToText` (`PlayerComponent.Points` (`self.PlayerComponent`))))))

(event `self.ShowCards`
  (bind _returnvalue (`PlayerComponent.GetCardIndexOfRole` (`self.PlayerComponent`) (`.RoleName` (break `Role` (`CPP_Piece.PieceRole` (`self.SavedPiece`))))))
  (`/Game/Player/Bp_WidgetPlayer.ShowCards` (`self.UI`) (`|GetArrayItem` _returnvalue) (`|GetArrayItem` _returnvalue 1)))

(event `self.HideCards`
  (`/Game/Player/Bp_WidgetPlayer.Hide Cards` (`self.UI`)))

(fn `UserConstructionScript`)
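; BP_Board is a tile board that marks a hardcoded set of grid tiles as occupied shortly after BeginPlay.
; ChangeTileOccupations looks up each coordinate with GetTileAt and sets IsOccupied on valid tiles.
; Occupied tiles get a dark red dynamic instance of M_PathfindMarking on their mesh, while clearing occupation leaves the material unchanged.
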(event `self.ReceiveBeginPlay`
  (`KismetSystemLibrary.Delay` 0.1)
  (`self.ChangeTileOccupations` (`|MakeArray` (make `2DVectorInt` 2 2) (make `2DVectorInt` 0 3) (make `2DVectorInt` 5 4) (make `2DVectorInt` 5 5) (make `2DVectorInt` 5 6)) true))

(fn `ChangeTileOccupations`
  (params (TileLocations :type "Array of 2DVectorInt Structure") (bOccupied :type Boolean))
  (for _array_element TileLocations
    (bind (_x _y) (break `2DVectorInt` _array_element))
    (bind _returnvalue (`self.GetTileAt` _x _y))
    (`/Engine/EditorBlueprintResources/StandardMacros.IsValid` _returnvalue
      (:`Is Valid`
        (bind _output_get (set `CPP_Tile.bIsOccupied` bOccupied _returnvalue))
        (if _output_get
          (bind _returnvalue_2 (`KismetMaterialLibrary.CreateDynamicMaterialInstance` "/Game/Resources/Materials/M_PathfindMarking.M_PathfindMarking"))
          (if true
            (`MaterialInstanceDynamic.SetVectorParameterValue` _returnvalue_2 "Color" (`KismetMathLibrary.MakeColor` 0.5)))
          (`PrimitiveComponent.SetMaterial` (`CPP_Tile.Mesh` _returnvalue) 0 _returnvalue_2))))))

(fn `UserConstructionScript`)
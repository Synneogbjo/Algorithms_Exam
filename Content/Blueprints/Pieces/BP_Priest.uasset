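; BP_Priest is the Priest game piece, handling its highlight glow and floating health-bar widget.
; BeginPlay hides the piece widget, caches it and tints its health bar dark purple.
; Highlight events toggle a flag and widget visibility, which Tick reads to turn the widget toward the camera and apply or clear a glow overlay material.
; The node setting the bar's fill from Health is unconnected and never runs.
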(event `self.ReceiveBeginPlay`
  (bind _returnvalue (`WidgetComponent.GetWidget` (`self.Widget`)))
  (if (`KismetSystemLibrary.IsValid` _returnvalue)
    (`Widget.SetVisibility` _returnvalue "Collapsed")
    (bind _asbp_piece_widget (cast `/Game/Blueprints/Pieces/WidgetPieces/bp_PieceWidget` _returnvalue))
    (bind _output_get (set `self.As Bp Piece Widget` _asbp_piece_widget))
    (`ProgressBar.SetFillColorAndOpacity` (`/Game/Blueprints/Pieces/WidgetPieces/bp_PieceWidget.HealthBar` _output_get) (struct :`R` 0.130277 :`G` 0.011232 :`B` 0.180555 :`A` 1.0))))

(event `self.ReceiveTick`
  (params (DeltaSeconds :type "Float (single-precision)"))
  (bind _widget (`self.Widget`))
  (if (`self.bIsHighlighted`)
    (`SceneComponent.K2_SetWorldRotation` _widget (`KismetMathLibrary.FindLookAtRotation` (`SceneComponent.K2_GetComponentLocation` _widget) (`PlayerCameraManager.GetCameraLocation` (`GameplayStatics.GetPlayerCameraManager` 0))) false false)
    (`MeshComponent.SetOverlayMaterial` (`self.MeshComponent`) "/Game/Material/M_GlowEffect.M_GlowEffect")
    (else
      (`MeshComponent.SetOverlayMaterial` (`self.MeshComponent`) null))))

(event `self.HighlightPiece`
  (set `self.bIsHighlighted` true)
  (`Widget.SetVisibility` (`self.As Bp Piece Widget`) "HitTestInvisible"))

(event `self.NotHighlightPiece`
  (set `self.bIsHighlighted` false)
  (`Widget.SetVisibility` (`self.As Bp Piece Widget`) "Collapsed"))

(fn `UserConstructionScript`)
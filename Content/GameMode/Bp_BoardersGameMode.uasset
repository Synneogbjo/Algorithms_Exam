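; Game mode for a two-player game that sets up the shared player UI at play start.
; BeginPlay adds the widget switcher to the viewport, shows the mouse cursor, then waits a tick before finding both player actors and handing each its child widget.
; Separate events activate each player's widget.
; EndGame prints a debug string and calls OnPlayerWin with an empty value.
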(event `self.ReceiveBeginPlay`
  (bind _returnvalue (`|GenericCreateObject` "/Game/Player/PlayerUI/Bp_PlayerWidgetSwitch.Bp_PlayerWidgetSwitch_C"))
  (bind _output_get (set `self.PlayersWigdet` _returnvalue))
  (`UserWidget.AddToViewport` _output_get 0)
  (set `PlayerController.bShowMouseCursor` true (`GameplayStatics.GetPlayerController` 0))
  (`KismetSystemLibrary.DelayUntilNextTick`)
  (`|ExecutionSequence`
    (:`then_0`
      (bind _returnvalue_2 (`GameplayStatics.GetActorOfClass` (`self.Player1Class`)))
      (if (`KismetSystemLibrary.IsValid` _returnvalue_2)
        (bind _output_get_2 (set `self.Player1_Ref` _returnvalue_2))
        (bind _asbp_player_1 (cast `/Game/Player/Bp_Player1` _output_get_2)
          (:`then`
            (set `/Game/Player/Bp_Player1.UI` (`/Game/Player/PlayerUI/Bp_PlayerWidgetSwitch.Bp_WidgetPlayer` (`self.PlayersWigdet`)) _asbp_player_1))
          (:`CastFailed`
            (`KismetSystemLibrary.PrintString` "failed" :!label _label)))
        (else
          (goto _label))))
    (:`then_1`
      (bind _returnvalue_3 (`GameplayStatics.GetActorOfClass` (`self.Player2Class`)))
      (if (`KismetSystemLibrary.IsValid` _returnvalue_3)
        (bind _output_get_3 (set `self.Player2_Ref` _returnvalue_3))
        (bind _asbp_player_2 (cast `/Game/Player/Bp_Player2` _output_get_3)
          (:`then`
            (set `/Game/Player/Bp_Player2.UI` (`/Game/Player/PlayerUI/Bp_PlayerWidgetSwitch.Bp_WidgetPlayer2` (`self.PlayersWigdet`)) _asbp_player_2))
          (:`CastFailed`
            (`KismetSystemLibrary.PrintString` "failed" :!label _label_2)))
        (else
          (goto _label_2))))))

(event `self.EndGame`
  (`KismetSystemLibrary.PrintString` "Hello")
  (`self.OnPlayerWin` ""))

(event `self.Player1WidgetSwitch`
  (`/Game/Player/Bp_WidgetPlayer.Player1ActiveWidget` (`/Game/Player/PlayerUI/Bp_PlayerWidgetSwitch.Bp_WidgetPlayer` (`self.PlayersWigdet`))))

(event `self.Player2WidgetSwitch`
  (`/Game/Player/Bp_WidgetPlayer2.Player2ActiveWidget` (`/Game/Player/PlayerUI/Bp_PlayerWidgetSwitch.Bp_WidgetPlayer2` (`self.PlayersWigdet`))))

(fn `UserConstructionScript`)